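; VR grabbable door Blueprint that swings on yaw to follow the motion controller holding its handle.
; A grab inside the handle's collision sphere stores the controller as the hand until that controller drops it.
; Each tick derives the door's clamped world yaw from the look-at angle between hand and door.
; The door locks only while nearly at zero yaw with its Keyhole not unlocked, and stays put when released.
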(event OnGrabbed(GrabComponent)
  (params (Self%20Reference :type Grab%20Component%20Object%20Reference) (MotionController :type Motion%20Controller%20Component%20Object%20Reference))
  (bind _handdle_collision (Variables|Default|GetHanddle%20Collision))
  (if (Utilities|Operators|EqualEqual (Transformation|GetWorldLocation MotionController) (Transformation|GetWorldLocation _handdle_collision) (Variables|/Script/Engine.SphereComponent|GetSphereRadius _handdle_collision))
    (Variables|Default|SetHand MotionController)))

(event OnDropped(GrabComponent)
  (params (Self%20Reference :type Grab%20Component%20Object%20Reference) (MotionController :type Motion%20Controller%20Component%20Object%20Reference))
  (if (== MotionController (Variables|Default|GetHand))
    (Variables|Default|SetHand 0)))

(event EventTick
  (params (DeltaSeconds :type Float%20%28single-precision%29))
  (bind _hand (Variables|Default|GetHand))
  (bind _door (Variables|Default|GetDoor))
  (Utilities|FlowControl|Sequence
    (:then_0
      ;[1 1 1] Locked?
      (if (and (not (Variables|/Game/Milk/Keyhold_BP.Keyhold_BP_C|GetUnlocked (Variables|Default|GetKeyhole))) (Math|Float|NearlyEqual(Float) (.yaw (Transformation|GetWorldRotation (Variables|Default|GetDoor))) 0.0 1e-06))
        (Variables|Default|SetLocked true)
        (else
          (Variables|Default|SetLocked false))))
    (:then_1
      ;[1 1 1] Set Door Rotation
      (if (not (Variables|Default|GetLocked))
        (Utilities|IsValid _hand
          (:Is%20Valid
            (Transformation|SetWorldRotation _door (Math|Rotator|MakeRotator 0.0 0.0 (Math|Float|ClampAngle (- (.yaw (Math|Rotator|FindLookatRotation (Transformation|GetWorldLocation _hand) (Transformation|GetWorldLocation _door))) 9e+01) -9e+01 9e+01)) false false))
          (:Is%20Not%20Valid
            (if (Math|Float|NearlyEqual(Float) (.yaw (Transformation|GetWorldRotation _door)) 0.0 1e-06)
              (Transformation|SetWorldRotation _door "0, 0, 0" false false))))))))

(fn ConstructionScript)