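; VR door Blueprint that swings while a motion controller grabs its GrabComponent.
; Grabbing stores the controller and starts a fast looping timer on UpdateRotation, and dropping clears both.
; UpdateRotation adds an X-axis offset, derived from the controller's relative location and its transform relative to GrabComponent, to the Scene component's yaw, clamped to ±90 degrees.
; An unconnected delayed Timeline reverse for rotating Door never runs.
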(event OnGrabbed(GrabComponent)
  (params (Self%20Reference :type Grab%20Component%20Object%20Reference) (MotionController :type Motion%20Controller%20Component%20Object%20Reference))
  (Variables|Default|SetMotion%20Controller MotionController)
  (bind _returnvalue (Utilities|Time|SetTimerbyFunctionName 0 "UpdateRotation" 0.01 true))
  (Variables|Default|SetTimer _returnvalue))

(event OnDropped(GrabComponent)
  (params (Self%20Reference :type Grab%20Component%20Object%20Reference) (MotionController :type Motion%20Controller%20Component%20Object%20Reference))
  (Utilities|Time|ClearandInvalidateTimerbyHandle (Variables|Default|GetTimer))
  (Variables|Default|SetMotion%20Controller 0))

(fn ConstructionScript)

(fn UpdateRotation
  (bind _motion_controller (Variables|Default|GetMotion%20Controller))
  (bind _scene (Variables|Default|GetScene))
  (bind _relativerotation (Variables|/Script/Engine.SceneComponent|GetRelativeRotation _scene))
  (Transformation|SetRelativeRotation _scene (Math|Rotator|MakeRotator (.roll _relativerotation) (.pitch _relativerotation) (Math|Float|Clamp(Float) (+ (.yaw _relativerotation) (.x (- (Variables|/Script/Engine.SceneComponent|GetRelativeLocation _motion_controller) (.location (Math|Transform|MakeRelativeTransform (Transformation|GetWorldTransform _motion_controller) (Transformation|GetWorldTransform (Variables|Default|GetGrabComponent))))))) -9e+01 9e+01)) false false))