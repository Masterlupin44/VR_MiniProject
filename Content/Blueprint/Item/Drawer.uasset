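; VR drawer item with two grab components, sliding two capsules along local Y as a motion controller pulls.
; Grabbing either component stores the controller and starts a looping timer, cleared on drop.
; Despite its name, UpdateRotation offsets both capsules by the controller's relative Y, clamping each between its spline's first two points.
; Both grabs share one controller and timer variable, and Spline1's point order is reversed for clamping.
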(event OnGrabbed(GrabComponent1)
  (params (Self%20Reference :type Grab%20Component%20Object%20Reference) (MotionController :type Motion%20Controller%20Component%20Object%20Reference))
  (Variables|Default|SetMotion%20Controler MotionController)
  (bind _returnvalue (Utilities|Time|SetTimerbyFunctionName 0 "UpdateRotation" 0.01 true))
  (Variables|Default|SetTimer _returnvalue))

(event OnDropped(GrabComponent1)
  (params (Self%20Reference :type Grab%20Component%20Object%20Reference) (MotionController :type Motion%20Controller%20Component%20Object%20Reference))
  (Utilities|Time|ClearandInvalidateTimerbyHandle (Variables|Default|GetTimer))
  (Variables|Default|SetMotion%20Controler 0))

(event OnGrabbed(GrabComponent2)
  (params (Self%20Reference :type Grab%20Component%20Object%20Reference) (MotionController :type Motion%20Controller%20Component%20Object%20Reference))
  (Variables|Default|SetMotion%20Controler MotionController)
  (bind _returnvalue (Utilities|Time|SetTimerbyFunctionName 0 "UpdateRotation" 0.01 true))
  (Variables|Default|SetTimer _returnvalue))

(event OnDropped(GrabComponent2)
  (params (Self%20Reference :type Grab%20Component%20Object%20Reference) (MotionController :type Motion%20Controller%20Component%20Object%20Reference))
  (Utilities|Time|ClearandInvalidateTimerbyHandle (Variables|Default|GetTimer))
  (Variables|Default|SetMotion%20Controler 0))

(fn ConstructionScript)

(fn UpdateRotation
  (bind _spline (Variables|Default|GetSpline))
  (bind _capsule (Variables|Default|GetCapsule))
  (bind _spline1 (Variables|Default|GetSpline1))
  (bind _capsule1 (Variables|Default|GetCapsule1))
  (bind _relativelocation (Variables|/Script/Engine.SceneComponent|GetRelativeLocation _capsule1))
  (bind _relativelocation_2 (Variables|/Script/Engine.SceneComponent|GetRelativeLocation _capsule))
  (Utilities|FlowControl|Sequence
    (:then_0
      (Transformation|SetRelativeLocation _capsule (Math|Vector|MakeVector (.x _relativelocation_2) (Math|Float|Clamp(Float) (+ (.y _relativelocation_2) (.y (.location (Math|Transform|MakeRelativeTransform (Transformation|GetWorldTransform (Variables|Default|GetMotion%20Controler)) (Transformation|GetWorldTransform (Variables|Default|GetCapsule)))))) (.y (Spline|GetLocationatSplinePoint _spline 0 "Local")) (.y (Spline|GetLocationatSplinePoint _spline 1 "Local"))) (.z _relativelocation_2)) false false))
    (:then_1
      (Transformation|SetRelativeLocation _capsule1 (Math|Vector|MakeVector (.x _relativelocation) (Math|Float|Clamp(Float) (+ (.y _relativelocation) (.y (.location (Math|Transform|MakeRelativeTransform (Transformation|GetWorldTransform (Variables|Default|GetMotion%20Controler)) (Transformation|GetWorldTransform (Variables|Default|GetCapsule1)))))) (.y (Spline|GetLocationatSplinePoint _spline1 1 "Local")) (.y (Spline|GetLocationatSplinePoint _spline1 0 "Local"))) (.z _relativelocation)) false false))))