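; Bin item that a motion controller can grab to tilt its Scene component.
; Grabbing stores the controller and starts a fast looping timer that calls UpdateRotation; dropping clears both.
; Each update adds an X offset, derived from the controller's relative location and its position relative to GrabComponent, to the current pitch, clamped to a narrow symmetric range while roll and yaw stay unchanged.
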(event OnGrabbed(GrabComponent)
  (params (Self%20Reference :type Grab%20Component%20Object%20Reference) (MotionController :type Motion%20Controller%20Component%20Object%20Reference))
  (Variables|Default|SetMotion%20Controler MotionController)
  (bind _returnvalue (Utilities|Time|SetTimerbyFunctionName 0 "UpdateRotation" 0.01 true))
  (Variables|Default|SetTimer _returnvalue))

(event OnDropped(GrabComponent)
  (params (Self%20Reference :type Grab%20Component%20Object%20Reference) (MotionController :type Motion%20Controller%20Component%20Object%20Reference))
  (Utilities|Time|ClearandInvalidateTimerbyHandle (Variables|Default|GetTimer))
  (Variables|Default|SetMotion%20Controler 0))

(event EventBeginPlay)

(event Collision|EventActorBeginOverlap
  (params (OtherActor :type Actor%20Object%20Reference)))

(event EventTick
  (params (DeltaSeconds :type Float%20%28single-precision%29)))

(fn ConstructionScript)

(fn UpdateRotation
  (bind _motion_controler (Variables|Default|GetMotion%20Controler))
  (bind _scene (Variables|Default|GetScene))
  (bind _relativerotation (Variables|/Script/Engine.SceneComponent|GetRelativeRotation _scene))
  (Transformation|SetRelativeRotation _scene (Math|Rotator|MakeRotator (.roll _relativerotation) (Math|Float|Clamp(Float) (+ (.pitch _relativerotation) (.x (- (Variables|/Script/Engine.SceneComponent|GetRelativeLocation _motion_controler) (.location (Math|Transform|MakeRelativeTransform (Transformation|GetWorldTransform _motion_controler) (Transformation|GetWorldTransform (Variables|Default|GetGrabComponent))))))) -2e+01 2e+01) (.yaw _relativerotation)) false false))